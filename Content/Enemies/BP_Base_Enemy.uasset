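; Base enemy character that provides player chasing, a sword attack, a patrol route and selectable movement speeds.
; ChasePlayer moves to the player with AI MoveTo, attacks on success, then re-calls itself after a delay, with no retry on failure.
; Attack plays the sword montage and fires OnAttackEnd on completion or interruption.
; Nothing in this graph starts the chase, while functions expose the patrol route and map speed states to walk speed.
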(event `self.ReceiveBeginPlay`)

(event `ChasePlayer`
  (`|AIMoveTo` self (0.0 0.0 0.0) (`GameplayStatics.GetPlayerCharacter` 0) 10.0
    (:`OnSuccess`
      (`self.Attack`)
      (`KismetSystemLibrary.Delay` 2.0)
      (`self.ChasePlayer`))))

(event `Attack`
  (`|PlayMontage` (`self.Mesh`) "/Game/Enemies/Skeleton/SwordMontage.SwordMontage"
    (:`OnCompleted`
      _)
    (:`OnInterrupted`
      _))
  (`self.OnAttackEnd`))

(fn `GetPatrolRoute`
  (returns (PatrolRoute :type "/Game/Enemies/PatrolRouteSkeleton Object Reference"))
  (return (`self.PatrolRoute`)))

(fn `SetMovementSpeed`
  (params (Speed :type "/Game/Enemies/Enums/E_MovementSpeed Enum" :default "NewEnumerator0"))
  (returns (SpeedValue :type "Float (double-precision)"))
  (set `CharacterMovementComponent.MaxWalkSpeed` (select `/Game/Enemies/Enums/E_MovementSpeed` Speed :`NewEnumerator1` 150.0 :`NewEnumerator2` 500.0 :!type "Float (single-precision)") (`self.CharacterMovement`))
  (return 0.0))

(fn `UserConstructionScript`)