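; BP_MyCharacter is a pirate captain player character with walking, jumping, mouse look and a sword attack.
; Movement axes feed movement input along the forward and right vectors of the control rotation, while mouse axes drive controller pitch and yaw.
; Left click plays the sword montage through a DoOnce that resets after a delay equal to the returned montage duration, preventing repeat attacks mid-swing.
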(event `InputAxis|Move Forward / Backward`
  (params (AxisValue :type "Float (single-precision)"))
  (bind (_returnvalue_roll _returnvalue_pitch _returnvalue_yaw) (`KismetMathLibrary.BreakRotator` (`self.GetControlRotation`)))
  ;[0 0 0] Movement
  (`self.AddMovementInput` (`KismetMathLibrary.GetForwardVector` (`KismetMathLibrary.MakeRotator` _returnvalue_roll _returnvalue_pitch _returnvalue_yaw)) AxisValue))

(event `InputAxis|Move Right / Left`
  (params (AxisValue :type "Float (single-precision)"))
  (bind (_returnvalue_roll _returnvalue_pitch _returnvalue_yaw) (`KismetMathLibrary.BreakRotator` (`self.GetControlRotation`)))
  ;[0 0 0] Movement
  (`self.AddMovementInput` (`KismetMathLibrary.GetRightVector` (`KismetMathLibrary.MakeRotator` _returnvalue_roll _returnvalue_pitch _returnvalue_yaw)) AxisValue))

(event `InputAction|Jump`
  (params (Key :type "Key Structure"))
  ;[0 0 0] Movement
  (:`Pressed`
    (`self.Jump`)))

(event `InputAxis|Look Up / Down Mouse`
  (params (AxisValue :type "Float (single-precision)"))
  ;[0 0 0] Camera
  (`self.AddControllerPitchInput` AxisValue))

(event `InputAxis|Turn Right / Left Mouse`
  (params (AxisValue :type "Float (single-precision)"))
  ;[0 0 0] Camera
  (`self.AddControllerYawInput` AxisValue))

(event `Key|LeftMouseButton`
  (params (Key :type "Key Structure"))
  (:`Pressed`
    (`/Engine/EditorBlueprintResources/StandardMacros.DoOnce` false :!label _label
      (:`Completed`
        (bind _returnvalue (`self.PlayAnimMontage` "/Game/Characters/PirateCaptain/SwordMontage.SwordMontage"))
        (`KismetSystemLibrary.Delay` _returnvalue)
        (goto _label :!via `Reset`)))))

(fn `UserConstructionScript`)